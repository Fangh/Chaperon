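; Clickable interaction actor that plays an assigned level sequence and disables itself when the sequence stops.
; While active, its Trigger reports cursor hover to the level's CursorManager, found at BeginPlay, and starts the sequence on click.
; On stop, it freezes the player at a hard-coded position with zero play rate, working around Restore State not working, then exits the cursor's interaction state.
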(event `self.ReceiveBeginPlay`
  (bind _outactors (`GameplayStatics.GetAllActorsOfClass` "/Game/BluePrints/CursorManager.CursorManager_C"))
  (set `self.CursorManager_Ref` (`|GetArrayItem` _outactors)))

(event `self.Trigger.OnBeginCursorOver`
  (params (TouchedComponent :type "PrimitiveComponent Object Reference"))
  (if (`self.IsActive`)
    (`/Game/BluePrints/CursorManager.OnEnterInteraction` (`self.CursorManager_Ref`))))

(event `self.Trigger.OnEndCursorOver`
  (params (TouchedComponent :type "PrimitiveComponent Object Reference"))
  (if (`self.IsActive`)
    (`/Game/BluePrints/CursorManager.OnExitInteraction` (`self.CursorManager_Ref`))))

(event `self.Trigger.OnClicked`
  (params (TouchedComponent :type "PrimitiveComponent Object Reference") (ButtonPressed :type "Key Structure" :default "AnyKey"))
  (if (`self.IsActive`)
    (bind _returnvalue (`LevelSequencePlayer.CreateLevelSequencePlayer` (`self.SequenceToPlay`)))
    (add `MovieSceneSequencePlayer.OnStop` _returnvalue (delegate `CustomEvent_0`))
    (`MovieSceneSequencePlayer.Play` _returnvalue)))

(event `CustomEvent_0`
  (`MovieSceneSequencePlayer.SetPlaybackPosition` (stale `self.Trigger.OnClicked` _returnvalue) 1.9) ; hack car Restore State = false ne fonctionne pas
  (`MovieSceneSequencePlayer.SetPlayRate` (stale `self.Trigger.OnClicked` _returnvalue) 0.0)
  (set `self.IsActive` false)
  (`/Game/BluePrints/CursorManager.OnExitInteraction` (`self.CursorManager_Ref`)))

(fn `UserConstructionScript`)