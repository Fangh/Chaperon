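; Clickable observation interactable that displays its Observation text when the player clicks its Trigger.
; Enable and disable events set IsActive and toggle Trigger collision, while BeginPlay caches the CursorManager (looked up twice) and applies an inactive starting state.
; When active, hover events notify the CursorManager, and a click prints the text, fires OnInteractionFinished and plays an optional sound at world origin.
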(event `EnableInteraction`
  (set `self.IsActive` true)
  (`PrimitiveComponent.SetCollisionEnabled` (`self.Trigger`) "QueryOnly"))

(event `DisableInteraction`
  (set `self.IsActive` false)
  (`PrimitiveComponent.SetCollisionEnabled` (`self.Trigger`) "NoCollision"))

(event `self.ReceiveBeginPlay`
  (`|ExecutionSequence`
    (:`then_0`
      (bind _outactors (`GameplayStatics.GetAllActorsOfClass` "/Game/BluePrints/CursorManager.CursorManager_C"))
      (set `self.CursorManager_Ref` (`|GetArrayItem` _outactors)))
    (:`then_1`
      (bind _outactors_2 (`GameplayStatics.GetAllActorsOfClass` "/Game/BluePrints/CursorManager.CursorManager_C"))
      (set `self.CursorManager_Ref` (`|GetArrayItem` _outactors_2)))
    (:`then_2`
      (if (not (`self.IsActive`))
        (`self.DisableInteraction`)))))

(event `self.Trigger.OnBeginCursorOver`
  (params (TouchedComponent :type "PrimitiveComponent Object Reference"))
  (if (`self.IsActive`)
    (`/Game/BluePrints/CursorManager.OnEnterInteraction` (`self.CursorManager_Ref`))))

(event `self.Trigger.OnEndCursorOver`
  (params (TouchedComponent :type "PrimitiveComponent Object Reference"))
  (if (`self.IsActive`)
    (`/Game/BluePrints/CursorManager.OnExitInteraction` (`self.CursorManager_Ref`))))

(event `self.Trigger.OnClicked`
  (params (TouchedComponent :type "PrimitiveComponent Object Reference") (ButtonPressed :type "Key Structure" :default "AnyKey"))
  (bind _soundtoplay (`self.SoundToPlay`))
  (if (`self.IsActive`)
    (`KismetSystemLibrary.PrintString` (`self.Observation`) true true (struct :`G` 0.66 :`B` 1.0 :`A` 1.0) 5.0)
    (`self.OnInteractionFinished`)
    (`/Engine/EditorBlueprintResources/StandardMacros.IsValid` _soundtoplay
      (:`Is Valid`
        (`GameplayStatics.PlaySoundAtLocation` self _soundtoplay)))))

(fn `UserConstructionScript`)