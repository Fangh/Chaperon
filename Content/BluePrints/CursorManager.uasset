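; CursorManager is an actor that draws a custom mouse cursor as a UMG widget.
; On BeginPlay it creates a Widget_Pointer, adds it to the viewport and sets the arrow cursor.
; Each Tick moves the widget to the DPI-scaled mouse position of player controller 0.
; OnEnterInteraction and OnExitInteraction events swap the widget's cursor between the hand and the arrow.
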(event `self.ReceiveBeginPlay`
  (bind _returnvalue (`|CreateWidget` "/Game/BluePrints/Widget_Pointer.Widget_Pointer_C" (`GameplayStatics.GetPlayerController` 0)))
  (bind _output_get (set `self.CursorWidget` _returnvalue))
  (`UserWidget.AddToViewport` _output_get 0)
  (set `/Game/BluePrints/Widget_Pointer.NewCursor` "/Game/Pointers/arrow-cursor.arrow-cursor" (`self.CursorWidget`)))

(event `self.ReceiveTick`
  (params (DeltaSeconds :type "Float (single-precision)"))
  (bind (_locationx _locationy) (`WidgetLayoutLibrary.GetMousePositionScaledByDPI` (`GameplayStatics.GetPlayerController` 0)))
  (`UserWidget.SetPositionInViewport` (`self.CursorWidget`) (`KismetMathLibrary.MakeVector2D` _locationx _locationy) false))

(event `OnEnterInteraction`
  (set `/Game/BluePrints/Widget_Pointer.NewCursor` "/Game/Pointers/hand-cursor.hand-cursor" (`self.CursorWidget`)))

(event `OnExitInteraction`
  (set `/Game/BluePrints/Widget_Pointer.NewCursor` "/Game/Pointers/arrow-cursor.arrow-cursor" (`self.CursorWidget`)))

(fn `UserConstructionScript`)