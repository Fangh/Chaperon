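; Dialogue actor that shows lines of text on screen in a DialogueBox widget created at BeginPlay.
; LaunchDialog takes a String Table ID as DialogID, caches that table's keys as the sentence order, adds the widget to the viewport and shows the first entry.
; Space increments SentenceIndex and sets the widget's text from the matching key, with no bounds check, index reset or widget removal.
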(event `self.ReceiveBeginPlay`
  (`self.EnableInput` (`GameplayStatics.GetPlayerController` 0))
  (bind _returnvalue (`|CreateWidget` "/Game/BluePrints/DialogueBox.DialogueBox_C"))
  (set `self.DialogWidget` _returnvalue))

(event `LaunchDialog`
  (params (DialogID :type Name))
  (bind _output_get (set `self.DialogID` DialogID))
  (bind _sentenceids (`self.CreateSentenceIDs` _output_get)) ; Fonction pour que ça prenne moins de place
  (set `self.SentenceIDs` _sentenceids)
  (`UserWidget.AddToViewport` (`self.DialogWidget`) 0)
  (`self.DisplayNextSentence` 0 (`self.DialogID`) (`self.SentenceIDs`)))

(event `Key|SpaceBar`
  (params (Key :type "Key Structure" :default "AnyKey"))
  (:`Pressed`
    (bind _result (`/Engine/EditorBlueprintResources/StandardMacros.IncrementInt` (`self.SentenceIndex`))
      (:`  `
        (`self.DisplayNextSentence` _result (`self.DialogID`) (`self.SentenceIDs`))))))

(fn `CreateSentenceIDs`
  (params (DialogID :type Name))
  (returns (SentenceIDs :type "Array of String"))
  (bind _output_get (set `self.SentenceIDs` (`KismetStringTableLibrary.GetKeysFromStringTable` DialogID)))
  (return _output_get))

(fn `DisplayNextSentence`
  (params (SentenceIndex :type Integer) (DialogId :type Name) (SentenceId :type "Array of String"))
  (set `/Game/BluePrints/DialogueBox.TextToDisplay` (`KismetTextLibrary.TextFromStringTable` DialogId (`|GetArrayItem` SentenceId SentenceIndex)) (`self.DialogWidget`)))

(fn `UserConstructionScript`)