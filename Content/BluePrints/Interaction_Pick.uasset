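; Interaction_Pick is a clickable pickup interaction that moves a world object into the player's inventory.
; Clicking its Trigger while active prints the observation text and calls OnInteractionFinished.
; It then adds one InventoryObjectID to the Inventory of the first ThirdPersonCharacter found via GetAllActorsOfClass, destroys ObjectToPick and deactivates itself.
; BeginPlay runs the parent logic and prints a debug greeting.
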(event `self.ReceiveBeginPlay`
  (`parent.ReceiveBeginPlay`)
  (`KismetSystemLibrary.PrintString` "Hello"))

(event `self.Trigger.OnClicked`
  (params (TouchedComponent :type "PrimitiveComponent Object Reference") (ButtonPressed :type "Key Structure" :default "AnyKey"))
  (if (`self.IsActive`)
    (`KismetSystemLibrary.PrintString` (`self.Observation`))
    (`self.OnInteractionFinished`)
    (bind _outactors (`GameplayStatics.GetAllActorsOfClass` "/Game/ThirdPersonBP/Blueprints/ThirdPersonCharacter.ThirdPersonCharacter_C"))
    (`BlueprintMapLibrary.Map_Add` (`/Game/ThirdPersonBP/Blueprints/ThirdPersonCharacter.Inventory` (`|GetArrayItem` _outactors)) (`self.inventoryObjectID`) 1)
    (`self.K2_DestroyActor` (`self.ObjectToPick`))
    (set `self.IsActive` false)))

(fn `UserConstructionScript`
  (`parent.UserConstructionScript`))